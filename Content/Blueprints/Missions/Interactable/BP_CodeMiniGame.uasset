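; BP_CodeMiniGame is a mission interactable for a code minigame that opens a door when its finish animation plays.
; PlayFinishAnimation records the door pivot's yaw, then a timeline rotates it 90 degrees in the negative yaw direction.
; When the timeline finishes, it calls CompleteMiniGameInteraction to end the interaction.
; GetMissionIndicatorPoint supplies the MissionIndicator component as the mission marker location.
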(event `self.PlayFinishAnimation`
  ;[0 0 0 0.5] Door animation
  (set `self.DoorRotationStartValue` (.yaw (`SceneComponent.RelativeRotation` (`self.DoorPoint`))))
  (bind (_direction _lerp) (`Timeline|Timeline`)
    (:`Update`
      (`SceneComponent.K2_SetRelativeRotation` (`self.DoorPoint`) (`KismetMathLibrary.MakeRotator` 0.0 0.0 (+ (`self.DoorRotationStartValue`) (* _lerp -90.0))) false false))
    (:`Finished`
      ;;[0 0 0 0.5] VERY IMPORTANT TO TRIGGER INTRERACTION END!!
      (`self.CompleteMiniGameInteraction`))))

(fn `GetMissionIndicatorPoint`
  (returns (ReturnValue :type "SceneComponent Object Reference"))
  (return (`self.MissionIndicator`)))

(fn `UserConstructionScript`)