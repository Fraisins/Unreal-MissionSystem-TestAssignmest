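; BP_Test_MissionGiver is a test actor that starts a mission when the player walks into its sphere trigger.
; On BeginPlay it binds to the mission subsystem's mission-added delegate and prints each added mission's ID.
; When the player character overlaps the sphere, it passes its MissionData to StartMission and prints whether the start succeeded or failed.
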(event `self.ReceiveBeginPlay`
  (add `MissionSubsystem.OnMissionAdded` (subsystem `MissionSubsystem`) (delegate `OnMissionAdded_Event`)))

(event `OnMissionAdded_Event`
  (params (MissionID :type Name))
  (`KismetSystemLibrary.PrintText` (`|FormatText` "{0} Mission Added!" MissionID)))

(event `self.Sphere.OnComponentBeginOverlap`
  (params (OverlappedComponent :type "PrimitiveComponent Object Reference") (OtherActor :type "Actor Object Reference") (OtherComp :type "PrimitiveComponent Object Reference") (OtherBodyIndex :type Integer) (bFromSweep :type Boolean) (SweepResult :type "HitResult Structure (by ref)"))
  (if (== OtherActor (`GameplayStatics.GetPlayerCharacter` 0))
    (bind _returnvalue (`MissionSubsystem.StartMission` (subsystem `MissionSubsystem`) (`self.MissionData`)))
    (if _returnvalue
      (`KismetSystemLibrary.PrintString` "MissionStarted!")
      (else
        (`KismetSystemLibrary.PrintString` "MissionFailed!")))))

(fn `UserConstructionScript`)